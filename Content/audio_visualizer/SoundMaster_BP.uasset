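; SoundMaster_BP is an audio visualizer controller that plays a sound on repeat and scales AudioElement_BP actors to its spectrum.
; The construction script gathers and shuffles those actors, so frequency bands map to them in random order.
; Playback-percent callbacks convert to time and sample normalized Constant-Q data (Audio Synesthesia), setting each valid actor's clamped Z scale.
; Tick restarts the audio whenever it stops.
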(event Custom|PlaybakChange
  (params (PlayingSoundWave :type Sound%20Wave%20Object%20Reference) (PlaybackPercent :type Float%20%28single-precision%29))
  (Variables|Default|SetPlayedTime (* PlaybackPercent (Variables|Default|GetDuration)))
  (for (_array_element _array_index) (Class|ConstantQNRT|GetNormalizedChannelConstantQatTime (Variables|Default|GetConstant_Ref) (Variables|Default|GetPlayedTime))
    ;[1 1 1] Cube shape
    (Utilities|IsValid (Utilities|Array|Get(acopy) (Variables|Default|GetAudioElement) _array_index)
      (:Is%20Valid
        (Transformation|SetWorldScale3D (Variables|/Script/Engine.Actor|GetRootComponent (Utilities|Array|Get(acopy) (Variables|Default|GetAudioElement) _array_index)) (Math|Vector|MakeVector 1.0 1.0 (Math|Float|Clamp(Float) (.z (* (Math|Conversions|ToVector(Float) _array_element) 2.0)) 0.7 1.3)))))))

(event EventBeginPlay
  (Audio|Components|Audio|SetSound (Variables|Default|GetAudio) (Variables|Default|GetNew%20Sound))
  (Variables|Default|SetDuration (Variables|/Script/Engine.SoundBase|GetDuration (Variables|Default|GetNew%20Sound)))
  (EventDispatchers|BindEventtoOnAudioPlaybackPercent (Variables|Default|GetAudio) (delegate Custom|PlaybakChange))
  (Audio|Components|Audio|Play (Variables|Default|GetAudio) 0.0))

(event EventTick
  (params (DeltaSeconds :type Float%20%28single-precision%29))
  (if (not (Audio|Components|Audio|IsPlaying (Variables|Default|GetAudio)))
    (Audio|Components|Audio|Play (Variables|Default|GetAudio) 0.0)))

(fn ConstructionScript
  (bind _outactors (Actor|GetAllActorsOfClass "/Game/audio_visualizer/AudioElement_BP.AudioElement_BP_C"))
  (bind _output_get (Variables|Default|SetAudioElement _outactors))
  (Utilities|Array|Shuffle _output_get))