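; HUD Blueprint that runs recurring Twitch vote rounds on screen, apparently to choose music changes.
; CreateWidget adds the TwitchUI widget to the viewport, starts the first round and sets a 30-second looping timer for later ones.
; Each round slides the panel in with a cowbell sound and counts down through a one-second Delay loop.
; At zero it closes voting, flags a pending music change and briefly shows the winner panel.
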(event Custom|TwitchUI
  (bind _ui_ref (Variables|Default|GetUI%20Ref))
  (bind _ui_ref_2 (Variables|Default|GetUI%20Ref))
  (bind _ui_ref_3 (Variables|Default|GetUI%20Ref))
  (bind _ui_ref_4 (Variables|Default|GetUI%20Ref))
  (Default|UpdateTime (Variables|Default|GetUI%20Ref))
  (Class|UserWidget|PlayAnimationForward _ui_ref_2 (Variables|/Game/TopDown/UI/TwitchUI.TwitchUI_C|GetSlideIn _ui_ref_2) 0.7 false)
  (Audio|PlaySound2D "/Game/Audio/SFXFiles/126995-Cowbell_ringing_brightly_x2.126995-Cowbell_ringing_brightly_x2" 0.9 1.0 0.0 0 0)
  (Variables|Default|SetIsVotingOn true)
  (Utilities|FlowControl|Delay 1.0 :!label _label)
  (Math|Integer|DecrementInt (Variables|Default|GetSecondsLeft)
    (:%20%20
      (Default|UpdateTime (Variables|Default|GetUI%20Ref))
      (if (> (Variables|Default|GetSecondsLeft) 0)
        (goto _label)
        (else
          (Class|UserWidget|PlayAnimationReverse _ui_ref_4 (Variables|/Game/TopDown/UI/TwitchUI.TwitchUI_C|GetSlideIn _ui_ref_4) 1.0 false)
          (Variables|Default|SetIsVotingOn false)
          (Variables|Default|SetIsMusicChangePending true)
          (Variables|Default|SetSecondsLeft (Variables|Default|Getvotetime))
          (Utilities|FlowControl|Delay 1.2)
          (Class|UserWidget|PlayAnimationForward _ui_ref_3 (Variables|/Game/TopDown/UI/TwitchUI.TwitchUI_C|GetWinnerSlideIn _ui_ref_3) 0.8 false)
          (Utilities|FlowControl|Delay 8.0)
          (Class|UserWidget|PlayAnimationReverse _ui_ref (Variables|/Game/TopDown/UI/TwitchUI.TwitchUI_C|GetWinnerSlideIn _ui_ref) 1.0 false))))))

(event Custom|Create%20Widget
  (Variables|Default|SetSecondsLeft (Variables|Default|Getvotetime))
  (bind _returnvalue (UserInterface|CreateWidget "/Game/TopDown/UI/TwitchUI.TwitchUI_C"))
  (bind _output_get (Variables|Default|SetUI%20Ref _returnvalue))
  (UserInterface|Viewport|AddtoViewport _output_get 0)
  (Utilities|Time|SetTimerbyEvent (delegate Custom|TwitchUI) 3e+01 true)
  (CallFunction|TwitchUI)
  (Default|UpdateTime (Variables|Default|GetUI%20Ref))
  (Class|UserWidget|PlayAnimationForward (Variables|Default|GetUI%20Ref) (Variables|/Game/TopDown/UI/TwitchUI.TwitchUI_C|GetSlideIn (Variables|Default|GetUI%20Ref)) 0.7 false)
  (Audio|PlaySound2D "/Game/Audio/SFXFiles/126995-Cowbell_ringing_brightly_x2.126995-Cowbell_ringing_brightly_x2" 0.9 1.0 0.0 0 0)
  (Variables|Default|SetIsVotingOn true)
  (Utilities|FlowControl|Delay 1.0 :!label _label)
  (Math|Integer|DecrementInt (Variables|Default|GetSecondsLeft)
    (:%20%20
      (Default|UpdateTime (Variables|Default|GetUI%20Ref))
      (if (> (Variables|Default|GetSecondsLeft) 0)
        (goto _label)
        (else
          (Class|UserWidget|PlayAnimationReverse (Variables|Default|GetUI%20Ref) (Variables|/Game/TopDown/UI/TwitchUI.TwitchUI_C|GetSlideIn (Variables|Default|GetUI%20Ref)) 1.0 false)
          (Variables|Default|SetIsVotingOn false)
          (Variables|Default|SetIsMusicChangePending true)
          (Variables|Default|SetSecondsLeft (Variables|Default|Getvotetime))
          (Utilities|FlowControl|Delay 1.2)
          (Class|UserWidget|PlayAnimationForward (Variables|Default|GetUI%20Ref) (Variables|/Game/TopDown/UI/TwitchUI.TwitchUI_C|GetWinnerSlideIn (Variables|Default|GetUI%20Ref)) 0.8 false)
          (Utilities|FlowControl|Delay 8.0)
          (Class|UserWidget|PlayAnimationReverse (Variables|Default|GetUI%20Ref) (Variables|/Game/TopDown/UI/TwitchUI.TwitchUI_C|GetWinnerSlideIn (Variables|Default|GetUI%20Ref)) 1.0 false))))))

(fn ConstructionScript)