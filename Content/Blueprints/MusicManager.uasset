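; MusicManager is a Blueprint that controls music playback through a Music audio component.
; SetSong switches tracks by passing a song index to the "Music Changes" parameter on that component, and StopSong stops it.
; A Debug function prints whether the separate 80BPM component is playing, while references to 100BPM and 120BPM sit unused.
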(event Collision|EventActorBeginOverlap
  (params (OtherActor :type Actor%20Object%20Reference)))

(fn ConstructionScript)

(fn SetSong
  (params (SongIndex :type Float%20%28double-precision%29))
  (Class|FMODAudioComponent|SetParameter (Variables|Default|GetMusic) "Music Changes" SongIndex))

(fn Debug
  (bind _returnvalue (Class|FMODAudioComponent|IsPlaying (Variables|Default|Get80_BPM)))
  (if _returnvalue
    (Development|PrintString "PLAYING")
    (else
      (Development|PrintString "STOPPED"))))

(fn StopSong
  (Class|FMODAudioComponent|Stop (Variables|Default|GetMusic)))